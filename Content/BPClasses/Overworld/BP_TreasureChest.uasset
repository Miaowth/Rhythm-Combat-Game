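; Interactable overworld treasure chest that grants items and money to the player inventory held by MyGameStateBase.
; DoInteract refuses if already looted or a set RequiresItem is missing, otherwise sets IsOpen on the chest's AnimBP.
; The Contents loop adds the first item and Money, then returns, so HasBeenLooted is set only when Contents is empty.
; Tooltip and interact control point are empty stubs.
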(fn `DoInteract`
  (params (Instigator :type "Actor Object Reference"))
  (returns (ReturnValue :type Boolean))
  (bind _requiresitem (`self.RequiresItem`))
  (bind _asmy_game_state_base (cast `MyGameStateBase` (`GameplayStatics.GetGameState`))
    (:`then`
      (if (`KismetSystemLibrary.IsValidClass` _requiresitem)
        (bind _playerinventory (`MyGameStateBase.PlayerInventory` _asmy_game_state_base))
        (bind (_index _returnvalue) (`Inventory.GetItemByClassRef` _playerinventory _requiresitem))
        (`/Engine/EditorBlueprintResources/StandardMacros.IsValid` _returnvalue
          (:`Is Valid`
            (if (`self.HasBeenLooted`) :!label _label
              (return false)
              (else
                (bind _asanim_bp_chest_01 (cast `/Game/Assets/SkeleMeshes/Chest_01/AnimBP_Chest_01` (`SkeletalMeshComponent.GetAnimInstance` (`self.SkeletalMesh`)))
                  (:`then`
                    (set `/Game/Assets/SkeleMeshes/Chest_01/AnimBP_Chest_01.isOpen` true _asanim_bp_chest_01))
                  (:`CastFailed`
                    _))
                (for _array_element (`self.Contents`)
                  (bind _returnvalue_2 (`Inventory.AddItemByItemAmt` _playerinventory _array_element))
                  (`Inventory.AddMoney` _playerinventory (`self.Money`))
                  (return _returnvalue_2))
                (set `self.HasBeenLooted` true)
                (return false))))
          (:`Is Not Valid`
            _))
        (else
          (goto _label))))
    (:`CastFailed`
      _))
  (return false))

(fn `GetInteractControlPoint`
  (params (Instigator :type "Actor Object Reference"))
  (returns (ReturnValue :type "Transform Structure"))
  (return))

(fn `GetTooltip`
  (returns (ReturnValue :type String))
  (return ""))

(fn `UserConstructionScript`)