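; BP_TownNPC is an overworld townsperson the player can interact with to start an Ink story.
; It creates its own Story from StoryAsset at BeginPlay.
; AI perception updates the Blackboard with the player pawn and whether it is currently seen.
; DoInteract turns the NPC toward the instigator and, if that is the player, has BP_MyHUD start the story, returning whether it did.
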(event `self.ReceiveBeginPlay`
  (bind _returnvalue (`Story.NewStory` (`self.StoryAsset`)))
  (set `self.Story` _returnvalue))

(event `self.AIPerception.OnTargetPerceptionUpdated`
  (params (Actor :type "Actor Object Reference") (Stimulus :type "AIStimulus Structure"))
  (bind _returnvalue (`AIBlueprintHelperLibrary.GetBlackboard` null))
  (if (== Actor (`GameplayStatics.GetPlayerPawn` 0))
    (`BlackboardComponent.SetValueAsObject` _returnvalue "PlayerCharacter" Actor)
    (`BlackboardComponent.SetValueAsBool` _returnvalue "CanSeePlayer" (`.bSuccessfullySensed` (break `AIStimulus` Stimulus)))))

(fn `DoInteract`
  (params (Instigator :type "Actor Object Reference"))
  (returns (ReturnValue :type Boolean))
  (`self.K2_SetActorRotation` (.rotation (`KismetAnimationLibrary.K2_LookAt` (`self.GetTransform`) (`self.K2_GetActorLocation` Instigator) (1.0 0.0 0.0) true (0.0 0.0 1.0))))
  (if (== Instigator (`GameplayStatics.GetPlayerPawn` 0))
    (bind _asbp_my_hud (cast `/Game/BPClasses/BP_MyHUD` (`PlayerController.GetHUD` (`GameplayStatics.GetPlayerController` 0)))
      (:`then`
        (`/Game/BPClasses/BP_MyHUD.StartInkStory` _asbp_my_hud (`self.Story`))
        (return true))
      (:`CastFailed`
        _)))
  (return false))

(fn `GetInteractControlPoint`
  (params (Instigator :type "Actor Object Reference"))
  (returns (ReturnValue :type "Transform Structure"))
  (return))

(fn `GetTooltip`
  (returns (ReturnValue :type String))
  (return ""))

(fn `UserConstructionScript`)