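; Rhythm-combat conductor that syncs scrolling UI notes to Wwise music.
; BeginCombat starts the music, whose beat and bar callbacks update the beat count, bar duration and scroll rate.
; Tick reads the playback position, spawns pending notes from the combat manager's four button arrays a few bars ahead onto two tracks, and scrolls them left.
; Miss detection is only a debug print on the top track.
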(event `self.ReceiveTick`
  (params (DeltaSeconds :type "Float (single-precision)"))
  (bind _rhythmuimanagerref (`self.RhythmUIManagerRef`))
  (bind _returnvalue (* (`self.BarsShownInAdvance`) (* -1 (* DeltaSeconds (`self.bpm`)))))
  (bind _returnvalue_2 (`AkGameplayStatics.GetSourcePlayPosition` (stale `self.BeginCombat` _output_get) :!label _label))
  (`self.SpawnChecking` _returnvalue_2
    (:`Completed`
      (for _array_element (`RhythmUI_Manager.TopTrackNoteArray` _rhythmuimanagerref)
        (bind _notesprite (`RhythmUI_Note.NoteSprite` _array_element))
        (`SceneComponent.K2_AddLocalOffset` _notesprite (`KismetMathLibrary.MakeVector` _returnvalue) false false)
        (bind _relativelocation_x (`KismetMathLibrary.BreakVector` (`SceneComponent.RelativeLocation` _notesprite)))
        (if (<= _relativelocation_x -500.0)
          (`/Engine/EditorBlueprintResources/StandardMacros.DoOnce` false
            (:`Completed`
              (`KismetSystemLibrary.PrintString` "Note Has Been Missed")))))
      (for _array_element_2 (`RhythmUI_Manager.BottomTrackNoteArray` _rhythmuimanagerref)
        (`SceneComponent.K2_AddLocalOffset` (`RhythmUI_Note.NoteSprite` _array_element_2) (`KismetMathLibrary.MakeVector` _returnvalue) false false)))))

(event `self.BeginCombat`
  (`KismetSystemLibrary.PrintString` "Hello")
  (`AkGameplayStatics.PostEvent` "/Game/WwiseAudio/Events/Default_Work_Unit/Play_ChangedChords.Play_ChangedChords" self 768 (delegate `NextBeat`))
  (bind _returnvalue (`AkGameObject.PostAssociatedAkEvent` :`self` (`self.CombatMusicAk`) :`CallbackMask` 1048576))
  (bind _output_get (set `self.CombatPlayingID` _returnvalue))
  (goto _label))

(event `NextBeat`
  (params (CallbackType :type "EAkCallbackType Enum" :default "EndOfEvent") (CallbackInfo :type "AkCallbackInfo Object Reference"))
  (bind _beatnum (`self.BeatNum`))
  (switch `EAkCallbackType` CallbackType
    (:`MusicSyncBeat`
      (bind _asak_music_sync_callback_info (cast `AkMusicSyncCallbackInfo` CallbackInfo))
      (`/Engine/EditorBlueprintResources/StandardMacros.IncrementInt` _beatnum
        (:`  `
          (`KismetSystemLibrary.PrintString` (`KismetStringLibrary.Conv_IntToString` _beatnum)))))
    (:`MusicSyncBar`
      (bind _asak_music_sync_callback_info_2 (cast `AkMusicSyncCallbackInfo` CallbackInfo))
      (bind (_currentposition _preentryduration _activeduration _postexitduration _remaininglookaheadtime _beatduration _barduration) (break `AkSegmentInfo` (`AkMusicSyncCallbackInfo.SegmentInfo` _asak_music_sync_callback_info_2)))
      (bind _returnvalue (`KismetMathLibrary.Conv_IntToDouble` _currentposition))
      (bind _output_get (set `self.BarDuration` (- _returnvalue (`self.LastBarStartPos`))))
      (bind _output_get_2 (set `self.LastBarStartPos` _returnvalue))
      (`KismetSystemLibrary.PrintString` (`KismetStringLibrary.Concat_StrStr` (`KismetStringLibrary.Conv_DoubleToString` (stale _output_get_3)) " next bar start"))
      (bind _output_get_3 (set `self.NextBarStartPos` (+ _output_get_2 _output_get)))
      (set `self.BeatLength` (/ _output_get (+ _barduration 1.0)))
      (set `self.BeatNum` 0)
      (`self.Updatebpm` _barduration))))

(fn `GetCombatMusicCurrentPlayPosition`
  (returns (NewParam :type Integer))
  (return 0))

(fn `SpawnUICheck`
  (params (InputPin :type "Float (double-precision)") (PatternNote :type "PatternNote Structure (by ref)") (RowNum :type Integer))
  (returns (IsNowSpawned :type Boolean) (UIElement :type "/Game/RhythmUI/BP_MyRhythmUI_Note Object Reference"))
  (bind (_isfinal _owningchar _posinms _isspawned) (break `PatternNote` PatternNote))
  (bind _rhythmuimanagerref (`self.RhythmUIManagerRef`))
  (bind _returnvalue (`self.GetTransform` (`RhythmUI_Manager.BottomTrackRef` _rhythmuimanagerref)))
  (bind _returnvalue_2 (`self.GetTransform` (`RhythmUI_Manager.TopTrackRef` _rhythmuimanagerref)))
  (if (and (<= _posinms (+ InputPin (* (`self.BarDuration`) (`self.BarsShownInAdvance`)))) (not _isspawned))
    (if (== 0 RowNum)
      (bind _returnvalue_3 (`|SpawnActorFromClass` "/Game/RhythmUI/BP_MyRhythmUI_Note.BP_MyRhythmUI_Note_C" (`KismetMathLibrary.MakeTransform` (`KismetMathLibrary.MakeVector` (+ (.x (.location _returnvalue_2)) 500.0) (.y (.location _returnvalue_2)) (.z (.location _returnvalue_2))) (.rotation _returnvalue_2) (.scale _returnvalue_2)) "Undefined" "OverrideRootScale" null null))
      (`KismetArrayLibrary.Array_Add` (`RhythmUI_Manager.TopTrackNoteArray` _rhythmuimanagerref) _returnvalue_3)
      (return true _returnvalue_3)
      (else
        (bind _returnvalue_4 (`|SpawnActorFromClass` "/Game/RhythmUI/BP_MyRhythmUI_Note.BP_MyRhythmUI_Note_C" (`KismetMathLibrary.MakeTransform` (`KismetMathLibrary.MakeVector` (+ (.x (.location _returnvalue)) 500.0) (.y (.location _returnvalue)) (.z (.location _returnvalue))) (.rotation _returnvalue) (.scale _returnvalue)) "Undefined" "OverrideRootScale" null null))
        (`KismetArrayLibrary.Array_Add` (`RhythmUI_Manager.BottomTrackNoteArray` _rhythmuimanagerref) _returnvalue_4)
        (return true _returnvalue_4)))
    (else
      (return false null))))

(fn `Updatebpm`
  (params (barduration :type "Float (double-precision)"))
  (set `self.bpm` (/ 60.0 barduration)))

(fn `UserConstructionScript`)