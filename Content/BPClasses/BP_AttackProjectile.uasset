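; BP_AttackProjectile is an attack projectile actor that travels from a starting point to a destination over a beat-based duration.
; CalculateSpeed doubles BeatDuration and derives Distance and Speed, though Tick reads neither of those two values.
; Tick accumulates delta time and linearly interpolates X and Y by elapsed time over BeatDuration, keeping the current Z.
; The interpolation alpha is not clamped, and no collision or end-of-travel logic is present.
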(event `self.CalculateSpeed`
  (bind _destinationpoint_location (`KismetMathLibrary.BreakTransform` (`self.DestinationPoint`)))
  (bind _startingpoint_location (`KismetMathLibrary.BreakTransform` (`self.StartingPoint`)))
  (bind _returnvalue (`KismetMathLibrary.VSize` (- _startingpoint_location _destinationpoint_location)))
  (set `self.BeatDuration` (* (`self.BeatDuration`) 2.0))
  (set `self.Distance` _returnvalue)
  (set `self.Speed` (/ _returnvalue (/ (`self.BeatDuration`) 10.0))))

(event `self.ReceiveTick`
  (params (DeltaSeconds :type "Float (single-precision)"))
  (bind (_returnvalue_x _returnvalue_y _returnvalue_z) (`KismetMathLibrary.BreakVector` (`self.K2_GetActorLocation`)))
  (bind _startingpoint (`self.StartingPoint`))
  (bind _destinationpoint (`self.DestinationPoint`))
  (bind _output_get (set `self.DeltaTracker` (+ DeltaSeconds (`self.DeltaTracker`))))
  (bind _returnvalue (/ _output_get (`self.BeatDuration`)))
  (`self.K2_SetActorLocation` (`KismetMathLibrary.MakeVector` (`KismetMathLibrary.Lerp` (.x (.location _startingpoint)) (.x (.location _destinationpoint)) _returnvalue) (`KismetMathLibrary.Lerp` (.y (.location _startingpoint)) (.y (.location _destinationpoint)) _returnvalue) _returnvalue_z)))

(fn `UserConstructionScript`)